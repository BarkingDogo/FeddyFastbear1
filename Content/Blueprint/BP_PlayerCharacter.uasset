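; First-person player character that presses in-world buttons and toggles a cheat menu.
; Mouse turn and look input drive the controller only while the menu is closed.
; Left click or E line-traces from the camera along its forward vector and calls PerformAction on any BP_Button hit, even with the menu open.
; Tab creates or removes the cheat menu widget, toggling the mouse cursor with it.
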(event `InputAxis|Turn` :overrideparent false
  (params (AxisValue :type "Float (single-precision)"))
  (if (not (`self.OpenedMenu?`))
    (`self.AddControllerYawInput` AxisValue)))

(event `InputAxis|LookUp` :overrideparent false
  (params (AxisValue :type "Float (single-precision)"))
  (if (not (`self.OpenedMenu?`))
    (`self.AddControllerPitchInput` AxisValue)))

(event `Key|LeftMouseButton`
  (params (Key :type "Key Structure"))
  (bind _firstpersoncamera (`self.FirstPersonCamera`))
  (bind _returnvalue (`SceneComponent.K2_GetComponentLocation` _firstpersoncamera))
  (:`Pressed`
    (bind _outhit (`KismetSystemLibrary.LineTraceSingle` :`Start` _returnvalue :`End` (+ _returnvalue (* (`SceneComponent.GetForwardVector` _firstpersoncamera) 3000.0)) :`TraceChannel` "TraceTypeQuery1" :`DrawDebugType` "ForOneFrame" :!label _label))
    (bind _asbp_button (cast `/Game/Blueprint/BP_Button` (`.HitActor` (`GameplayStatics.BreakHitResult` _outhit))))
    (`/Game/Blueprint/BP_Button.PerformAction` _asbp_button)))

(event `Key|E`
  (params (Key :type "Key Structure"))
  (:`Pressed`
    (goto _label)))

(event `Key|Tab`
  (params (Key :type "Key Structure"))
  (:`Pressed`
    (if (`self.OpenedMenu?`)
      (`Widget.RemoveFromParent` (`self.TempWidget`))
      (set `PlayerController.bShowMouseCursor` false (`GameplayStatics.GetPlayerController` 0))
      (set `self.OpenedMenu?` false)
      (else
        (bind _returnvalue (`|CreateWidget` "/Game/Blueprint/Widget_CheatMenuProto.Widget_CheatMenuProto_C" (`GameplayStatics.GetPlayerController` 0)))
        (bind _output_get (set `self.TempWidget` _returnvalue))
        (`UserWidget.AddToViewport` _output_get 0)
        (set `PlayerController.bShowMouseCursor` true (`GameplayStatics.GetPlayerController` 0))
        (set `self.OpenedMenu?` true)))))

(fn `UserConstructionScript`)