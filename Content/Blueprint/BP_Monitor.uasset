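; BP_Monitor is a monitor actor that pairs with BP_CCTV_Camera actors and blanks its screen when the active camera is off.
; Its construction script gathers all cameras in the level and selects the first as active, without activating it.
; Tick polls that camera's on state and, only on changes, toggles the Disable material parameter on the screen plane.
; SwitchCamera deactivates the current camera and activates the new one.
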(event `self.ReceiveTick`
  (params (DeltaSeconds :type "Float (single-precision)"))
  (`/Engine/EditorBlueprintResources/StandardMacros.IsValid` (`self.ActiveCamera`)
    (:`Is Valid`
      (if (`/Game/Blueprint/BP_CCTV_Camera.IsCameraOn?` (`self.ActiveCamera`))
        (if (not (`self.MonitorTurnedOn?`))
          (`MeshComponent.SetScalarParameterValueOnMaterials` (`self.Plane`) "Disable" 0.0)
          (set `self.MonitorTurnedOn?` true))
        (elif (`self.MonitorTurnedOn?`)
          (`MeshComponent.SetScalarParameterValueOnMaterials` (`self.Plane`) "Disable" 1.0)
          (set `self.MonitorTurnedOn?` false))))))

(fn `SwitchCamera`
  (params (NewCamera :type "/Game/Blueprint/BP_CCTV_Camera Object Reference"))
  (`/Game/Blueprint/BP_CCTV_Camera.DeactivateCamera` (`self.ActiveCamera`))
  (bind _output_get (set `self.ActiveCamera` NewCamera))
  (`/Game/Blueprint/BP_CCTV_Camera.ActivateCamera` _output_get))

(fn `UserConstructionScript`
  (bind _outactors (`GameplayStatics.GetAllActorsOfClass` "/Game/Blueprint/BP_CCTV_Camera.BP_CCTV_Camera_C"))
  (bind _output_get (set `self.AllCameras` _outactors))
  (if (not (== (`KismetArrayLibrary.Array_Length` _output_get) 0))
    (bind _output_get_2 (set `self.ActiveCamera` (`|GetArrayItem` (`self.AllCameras`))))))