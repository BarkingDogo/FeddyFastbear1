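; BP_LightButton is a button that switches an attached light and controls a sound along with it.
; PerformAction calls ToogleLights on AttachedLight and branches on its result.
; A true result creates and plays PerformSound as a 2D sound, storing it in NewVar0, and a false result stops that stored sound.
; The event graph holds only disabled default events, and the construction script only calls its parent.
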(fn `PerformAction`
  (bind _newparam (`/Game/Blueprint/BP_Light.ToogleLights` (`self.AttachedLight`)))
  (if _newparam
    (bind _returnvalue (`GameplayStatics.CreateSound2D` (`self.PerformSound`) 1.0 1.0 0.0 null))
    (set `self.NewVar_0` _returnvalue)
    (`AudioComponent.Play` _returnvalue 0.0)
    (else
      (`AudioComponent.Stop` (`self.NewVar_0`)))))

(fn `UserConstructionScript`
  (`parent.UserConstructionScript`))