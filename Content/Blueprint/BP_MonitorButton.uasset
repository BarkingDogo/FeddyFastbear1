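; BP_MonitorButton is a button actor that switches a monitor's view to the camera attached to it.
; Its construction script caches the first BP_Monitor found and labels the button with the camera's BP_NameComponent name, printing a leftover "Hello" message.
; PerformAction calls SwitchCamera on that monitor with the attached camera and plays a sound at the button's location.
; The event graph holds only disabled default events.
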(fn `PerformAction`
  (`/Game/Blueprint/BP_Monitor.SwitchCamera` (`self.Monitor`) (`self.AttachedCamera`))
  (`GameplayStatics.PlaySoundAtLocation` (`self.PerformSound`) (`self.K2_GetActorLocation`) (struct) 1.0 1.0 0.0 null null null))

(fn `UserConstructionScript`
  (bind _returnvalue (`self.GetComponentByClass` (`self.AttachedCamera`) "/Game/Blueprint/BP_NameComponent.BP_NameComponent_C"))
  (`|ExecutionSequence`
    (:`then_0`
      (bind _outactors (`GameplayStatics.GetAllActorsOfClass` "/Game/Blueprint/BP_Monitor.BP_Monitor_C"))
      (set `self.Monitor` (`|GetArrayItem` _outactors)))
    (:`then_1`
      (`/Engine/EditorBlueprintResources/StandardMacros.IsValid` _returnvalue
        (:`Is Valid`
          (`TextRenderComponent.K2_SetText` (`self.CameraName`) (`/Game/Blueprint/BP_NameComponent.ObjectName` _returnvalue))
          (`KismetSystemLibrary.PrintString` "Hello"))))))