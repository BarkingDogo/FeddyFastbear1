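; BP_Door is a door actor whose ToggleDoor function switches the Cube between open and closed using the DoorClosed flag.
; Opening snaps the Cube upward with a local offset, while closing plays a timeline from the start and sets the flag immediately.
; The EventGraph's timeline update maps its track to the Cube's relative height, though that timeline node has no wired input.
; Leftover offset nodes are unconnected, including an instant downward close.
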(fn `ToggleDoor`
  (if (`self.DoorClosed?`)
    (`SceneComponent.K2_AddLocalOffset` (`self.Cube`) (0.0 0.0 250.0) false false)
    (set `self.DoorClosed?` false)
    (else
      (`TimelineComponent.PlayFromStart` (`self.Timeline_0`))
      (set `self.DoorClosed?` true))))

(fn `UserConstructionScript`)