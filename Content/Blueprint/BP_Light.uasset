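; Toggleable point light Blueprint with a subtle flicker driven by a timeline.
; ToogleLights switches between zero and the LighsParamet intensity, stops or restarts the timeline, and returns the new on/off state.
; Timeline updates scale that intensity by a curve and a random modifier, which is re-rolled within a narrow range when the timeline finishes.
; The timeline node has no wired inputs in the event graph, and Tick is empty.
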(event `self.ReceiveTick`
  (params (DeltaSeconds :type "Float (single-precision)")))

(fn `ToogleLights`
  (returns (NewParam :type Boolean))
  (if (`self.IsLightsOn?`)
    (`TimelineComponent.Stop` (`self.Timeline_0`))
    (`LightComponent.SetIntensity` (`self.PointLight`) 0.0)
    (bind _output_get (set `self.IsLightsOn?` false))
    (return _output_get)
    (else
      (`LightComponent.SetIntensity` (`self.PointLight`) (`self.LighsParamet`))
      (`TimelineComponent.PlayFromStart` (`self.Timeline_0`))
      (bind _output_get_2 (set `self.IsLightsOn?` true))
      (return _output_get_2))))

(fn `UserConstructionScript`)