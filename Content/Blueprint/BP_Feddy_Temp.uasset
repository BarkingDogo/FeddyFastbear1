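; Temporary Freddy animatronic that advances along tagged BP_TravelPoint actors in Priority order, in a Five Nights at Freddy's style.
; The first Tick places it at the starting point; each later Tick rolls a d20 against AIDifficult to decide whether it moves.
; At a Point.Final point, a successful roll loops it back to the start.
; MoveToNextPoint relocates the actor and turns off active cameras attached to the old and new points.
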(event `self.ReceiveTick`
  (params (DeltaSeconds :type "Float (single-precision)"))
  (bind _newvar_0 (`self.NewVar_0`))
  (if (`self.FirstTick?`)
    (set `self.FirstTick?` false)
    (bind _outactors (`GameplayStatics.GetAllActorsOfClass` "/Game/Blueprint/BP_TravelPoint.BP_TravelPoint_C"))
    (for _array_element _outactors
      (if (and (`self.ActorHasTag` _array_element "Animatronics.Freddy") (== (`/Game/Blueprint/BP_TravelPoint.Priority` _array_element) 0))
        (`self.MoveToNextPoint` _array_element)
        (break)))
    (else
      (set `self.NewVar_0` (`KismetMathLibrary.RandomIntegerInRange` 1 20))
      (`KismetSystemLibrary.PrintString` (`KismetStringLibrary.Conv_IntToString` _newvar_0))
      (if (>= (`self.AI_Difficult`) _newvar_0)
        (if (`self.ActorHasTag` (`self.CurrentPoint`) "Point.Final")
          (set `self.Priority` -1)
          (bind _outactors_2 (`GameplayStatics.GetAllActorsOfClass` "/Game/Blueprint/BP_TravelPoint.BP_TravelPoint_C"))
          (for _array_element_2 _outactors_2
            (if (and (`self.ActorHasTag` _array_element_2 "Animatronics.Freddy") (== (`/Game/Blueprint/BP_TravelPoint.Priority` _array_element_2) 0))
              (`self.MoveToNextPoint` _array_element_2)
              (break)))
          (else
            (bind _outactors_3 (`GameplayStatics.GetAllActorsOfClass` "/Game/Blueprint/BP_TravelPoint.BP_TravelPoint_C"))
            (for _array_element_3 _outactors_3
              (if (and (`self.ActorHasTag` _array_element_3 "Animatronics.Freddy") (== (`/Game/Blueprint/BP_TravelPoint.Priority` _array_element_3) (+ (`self.Priority`) 1)))
                (`self.MoveToNextPoint` _array_element_3)
                (break)))))))))

(fn `MoveToNextPoint`
  (params (NewPoint :type "/Game/Blueprint/BP_TravelPoint Object Reference"))
  (bind _attachedcamera (`/Game/Blueprint/BP_TravelPoint.AttachedCamera` (`self.CurrentPoint`)))
  (bind _attachedcamera_2 (`/Game/Blueprint/BP_TravelPoint.AttachedCamera` (`self.CurrentPoint`)))
  (`/Engine/EditorBlueprintResources/StandardMacros.IsValid` (`self.CurrentPoint`)
    (:`Is Valid`
      (`|ExecutionSequence`
        (:`then_0`
          (if (`/Game/Blueprint/BP_CCTV_Camera.ActiveCamera?` _attachedcamera_2)
            (`/Game/Blueprint/BP_CCTV_Camera.TurnOffCamera` _attachedcamera_2)))
        (:`then_1`
          (bind _output_get (set `self.CurrentPoint` NewPoint :!label _label))
          (`/Engine/EditorBlueprintResources/StandardMacros.IncrementInt` (`self.Priority`)
            (:`  `
              (`self.K2_SetActorLocation` (`self.K2_GetActorLocation` _output_get))
              (if (`/Game/Blueprint/BP_CCTV_Camera.ActiveCamera?` _attachedcamera)
                (`/Game/Blueprint/BP_CCTV_Camera.TurnOffCamera` _attachedcamera)))))))
    (:`Is Not Valid`
      (goto _label))))

(fn `UserConstructionScript`)